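; BP_GradientCreator is an editor tool actor that bakes anime toon-shading gradients into the RT_GradeintRender render target.
; Its construction script resets an Update flag, creates a dynamic M_GradientCreator material on a preview plane and passes it to Generate.
; Generate pushes fresnel, rim and banded-shading variables into the material, with rim smoothness raised to the fifth power, then draws it to the render target.
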(event Custom|Generate
  (params (Material :type Material%20Instance%20Dynamic%20Object%20Reference))
  (Variables|Default|SetDynamicMaterial Material)
  (Rendering|Material|SetScalarParameterValue (Variables|Default|GetDynamicMaterial) "FresnelPower" (Variables|Fresnel|GetFresnelPower) :!class /Script/Engine.MaterialInstanceDynamic)
  (Rendering|Material|SetScalarParameterValue (Variables|Default|GetDynamicMaterial) "FresnelScale" (Variables|Fresnel|GetFresnelScale) :!class /Script/Engine.MaterialInstanceDynamic)
  (Rendering|Material|SetScalarParameterValue (Variables|Default|GetDynamicMaterial) "RimWidth" (Variables|Rim|GetRimWidth) :!class /Script/Engine.MaterialInstanceDynamic)
  (Rendering|Material|SetScalarParameterValue (Variables|Default|GetDynamicMaterial) "RimAngle" (Variables|Rim|GetRimAngle) :!class /Script/Engine.MaterialInstanceDynamic)
  (Rendering|Material|SetScalarParameterValue (Variables|Default|GetDynamicMaterial) "RimScale" (Variables|Rim|GetRimScale) :!class /Script/Engine.MaterialInstanceDynamic)
  (Rendering|Material|SetScalarParameterValue (Variables|Default|GetDynamicMaterial) "RimSmooth" (Math|Float|Power (Variables|Rim|GetRimSmooth) 5.0) :!class /Script/Engine.MaterialInstanceDynamic)
  (Rendering|Material|SetScalarParameterValue (Variables|Default|GetDynamicMaterial) "Dark" (Variables|Shading|GetShadingDark) :!class /Script/Engine.MaterialInstanceDynamic)
  (Rendering|Material|SetScalarParameterValue (Variables|Default|GetDynamicMaterial) "Slope" (Variables|Shading|GetShadingSlope) :!class /Script/Engine.MaterialInstanceDynamic)
  (Rendering|Material|SetScalarParameterValue (Variables|Default|GetDynamicMaterial) "Gaps" (Variables|Shading|GetShadingGaps) :!class /Script/Engine.MaterialInstanceDynamic)
  (Rendering|Material|SetScalarParameterValue (Variables|Default|GetDynamicMaterial) "Shift" (Variables|Shading|GetShadingShift) :!class /Script/Engine.MaterialInstanceDynamic)
  (Rendering|Material|SetScalarParameterValue (Variables|Default|GetDynamicMaterial) "Divisions" (Variables|Shading|GetShadingDivisions) :!class /Script/Engine.MaterialInstanceDynamic)
  (Rendering|DrawMaterialtoRenderTarget "/Game/EY_Project/Other_Matrial/AnimeToonShading/Gradients/RT_GradeintRender.RT_GradeintRender" (Variables|Default|GetDynamicMaterial)))

(fn ConstructionScript
  (Variables|Rendering|SetUpdate false)
  (bind _returnvalue (Rendering|Material|CreateDynamicMaterialInstance (Variables|Default|GetPlane) 0 "/Game/EY_Project/Other_Matrial/AnimeToonShading/Gradients/M_GradientCreator.M_GradientCreator" "None" :!class /Script/Engine.PrimitiveComponent))
  (CallFunction|Generate _returnvalue))